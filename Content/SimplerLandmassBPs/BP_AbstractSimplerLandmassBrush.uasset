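; Abstract base Blueprint for Simpler Landmass landscape brushes, providing update requests, update throttling and an enable toggle.
; Update timestamps are cached per brush in a BP_SimplerLandmassBrushDataManager actor, found or spawned on demand, because ordinary member variables often lose their values.
; The delay check compares the current time to that cached timestamp plus a minimum delay, and the timestamp is reset separately.
; Toggling the brush requests a landscape update.
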(fn ConstructionScript)

(fn GetBrushDataManager
  (Utilities|FlowControl|Sequence
    (:then_0
      ;[1 1 1] Creates a "random" actor that is used as cache. Normal non-public, non-readonly variables seem to get "lost" often.
      (Utilities|IsValid (Variables|Workaround|GetBrush%20Data%20Manager)
        (:Is%20Not%20Valid
          (bind _outactors (Actor|GetAllActorsOfClass "/Game/Dependencies/Workaround/BP_SimplerLandmassBrushDataManager.BP_SimplerLandmassBrushDataManager_C"))
          (if (>= (Utilities|Array|LastIndex _outactors) 0)
            (Variables|Workaround|SetBrush%20Data%20Manager (Utilities|Array|Get(acopy) _outactors (Utilities|Array|LastIndex _outactors)))
            (else
              (bind _returnvalue (EditorScripting|LevelUtility|SpawnActorfromClass "/Game/Dependencies/Workaround/BP_SimplerLandmassBrushDataManager.BP_SimplerLandmassBrushDataManager_C" :!class /Script/EditorScriptingUtilities.EditorLevelLibrary))
              (Variables|Workaround|SetBrush%20Data%20Manager _returnvalue))))))
    (:then_1
      (Utilities|FlowControl|Sequence
        (:then_0
          ;[1 1 1] End
          (return (Variables|Workaround|GetBrush%20Data%20Manager)))))))

(fn TriggerLandscapeUpdate
  (Landscape|RequestLandscapeUpdate))

(fn IsUpdateDelayPassed
  ;[1 1 1] Checks against a cached timestamp. The timestamp caching needs to be triggered separately.
  (return (> (Math|DateTime|Now) (+ (Default|GetCachedUpdateTimestamp (Workaround|GetBrushDataManager) self) (Math|Timespan|MakeTimespan 0 0 0 0 (Variables|Efficiency|GetMinimum%20Update%20Delay%20%28ms%29))))))

(fn ResetUpdateDelay
  ;[1 1 1] Reset last update timestamp
  (Default|CacheUpdateTimestamp (Workaround|GetBrushDataManager) self))

(fn Enable/DisableBrush
  ;[1 1 1] Disable brush
  (Variables|Triggers|SetIs%20Brush%20Enabled (not (Variables|Triggers|GetIs%20Brush%20Enabled)))
  (Triggers|TriggerLandscapeUpdate))