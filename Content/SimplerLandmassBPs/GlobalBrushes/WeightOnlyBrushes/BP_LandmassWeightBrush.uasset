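; Landmass brush that paints landscape weightmap layers from a list of named materials, passing the heightmap through unchanged.
; The heightmap pass refreshes cached MIDs and feeds them the height render target and actor position.
; Each weightmap pass clears a cached render target and draws that layer's MID, plus any per-layer debug target.
; An update delay throttles rendering by returning the cached result, and layer mappings rebuild when materials change.
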(fn ConstructionScript)

(fn Render
  (params (InIsHeightmap :type Boolean) (InCombinedResult :type Texture%20Render%20Target%202D%20Object%20Reference) (InWeightmapLayerName :type Name%20%28by%20ref%29 :default "None"))
  (bind _current_rt (Variables|Internal|GetCurrent%20RT))
  (Utilities|FlowControl|Sequence
    (:then_0
      ;[1 1 1] 1. Local Variables
      (LocalVariables|SetIn%20Is%20Heightmap InIsHeightmap)
      (LocalVariables|SetIn%20Combined%20Result InCombinedResult)
      (LocalVariables|SetIn%20Weightmap%20Layer%20Name InWeightmapLayerName))
    (:then_1
      (Utilities|FlowControl|Sequence
        (:then_0
          ;[1 1 1] Early return for if disabled
          (if (not (Variables|Default|GetIs%20Brush%20Enabled))
            (return (LocalVariables|GetIn%20Combined%20Result))))
        (:then_1
          (Utilities|FlowControl|Sequence
            (:then_0
              ;[1 1 1] Dont update too often, Return probably existing RT from last time
              (if (not (CallFunction|IsUpdateDelayPassed))
                (return (Default|GetCachedRenderTarget (CallFunction|GetBrushDataManager) self))))
            (:then_1
              (Utilities|FlowControl|Sequence
                (:then_0
                  ;[1 1 1] 2. Check parameters
                  (if (== 0 (Utilities|Array|Length (Variables|Parameters|GetMaterials)))
                    (return (LocalVariables|GetIn%20Combined%20Result))
                    (else
                      (for _array_element (Variables|Parameters|GetMaterials)
                        (if (not (and (Utilities|Name|NotEqual(Name) (.Name (Utilities|Struct|BreakStruct_LandmassWeightBrushMaterials _array_element)) "None") (Utilities|IsValid (.Material (Utilities|Struct|BreakStruct_LandmassWeightBrushMaterials _array_element)))))
                          (return (LocalVariables|GetIn%20Combined%20Result)))))))
                (:then_1
                  (Utilities|FlowControl|Sequence
                    (:then_0
                      ;[1 1 1] 3. Reset Internal state / Set Variables
                      (CallFunction|ResetInternalState (LocalVariables|GetIn%20Is%20Heightmap) (LocalVariables|GetIn%20Combined%20Result) (LocalVariables|GetIn%20Weightmap%20Layer%20Name)))
                    (:then_1
                      (Utilities|FlowControl|Sequence
                        (:then_0
                          ;[1 1 1] 5. Setup Height Related Material Parameters in all Weight MIDs
                          (if (LocalVariables|GetIn%20Is%20Heightmap)
                            (bind _values (Utilities|Map|Values (Variables|Internal|GetCurrent%20MID%20by%20Material)))
                            (CallFunction|SetupHeightRelatedMaterialParameters (LocalVariables|GetIn%20Combined%20Result) _values)
                            ;[1 1 1] 6. Early return for heightmaps
                            (return (LocalVariables|GetIn%20Combined%20Result))))
                        (:then_1
                          (Utilities|FlowControl|Sequence
                            (:then_0
                              ;[1 1 1] 7. Setup parameters of current MID
                              (CallFunction|SetupWeightRelatedMaterialParameters (Variables|Internal|GetCurrent%20MID)))
                            (:then_1
                              (Utilities|FlowControl|Sequence
                                (:then_0
                                  ;[1 1 1] 8. Explicitly show debug messages for missing RT or MID
                                  (if (not (and (Utilities|IsValid (Variables|Internal|GetCurrent%20MID)) (Utilities|IsValid (Variables|Internal|GetCurrent%20RT))))
                                    (Development|PrintString (Utilities|String|Append "Invalid state while drawing in " (Utilities|GetDisplayName self)) true true "(R=1.000000,G=0.416440,B=0.000000,A=1.000000)" 5.0)))
                                (:then_1
                                  (Utilities|FlowControl|Sequence
                                    (:then_0
                                      ;[1 1 1] 9. Draw debug target
                                      (if (.ReturnValue (Utilities|Map|Find (Variables|Debug|GetDebug%20Render%20Targets%20by%20Layer) (LocalVariables|GetIn%20Weightmap%20Layer%20Name)))
                                        (Rendering|ClearRenderTarget2D (.Value (Utilities|Map|Find (Variables|Debug|GetDebug%20Render%20Targets%20by%20Layer) (LocalVariables|GetIn%20Weightmap%20Layer%20Name))))
                                        (Rendering|DrawMaterialtoRenderTarget (.Value (Utilities|Map|Find (Variables|Debug|GetDebug%20Render%20Targets%20by%20Layer) (LocalVariables|GetIn%20Weightmap%20Layer%20Name))) (Variables|Internal|GetCurrent%20MID))))
                                    (:then_1
                                      (Utilities|FlowControl|Sequence
                                        (:then_0
                                          ;[1 1 1] 10. Draw Final Weight MID
                                          (Rendering|ClearRenderTarget2D _current_rt)
                                          (Rendering|DrawMaterialtoRenderTarget _current_rt (Variables|Internal|GetCurrent%20MID)))
                                        (:then_1
                                          (Utilities|FlowControl|Sequence
                                            (:then_0
                                              ;[1 1 1] End
                                              (CallFunction|ResetUpdateDelay)
                                              (return (Variables|Internal|GetCurrent%20RT)))))))))))))))))))))))))

(fn ResetInternalState
  (params (Is%20Heightmap :type Boolean%20%28by%20ref%29) (Combined%20Result :type Texture%20Render%20Target%202D%20Object%20Reference%20%28by%20ref%29) (Weightmap%20Layer%20Name :type Name%20%28by%20ref%29))
  (bind _brush_data_manager (CallFunction|GetBrushDataManager))
  (bind _affectedweightmaplayers (Variables|Default|GetAffectedWeightmapLayers))
  (bind _current_mid_by_material (Variables|Internal|GetCurrent%20MID%20by%20Material))
  (Utilities|FlowControl|Sequence
    (:then_0
      ;[1 1 1] Local Variables
      (LocalVariables|SetIn%20Is%20Heightmap Is%20Heightmap)
      (LocalVariables|SetIn%20Combined%20Result Combined%20Result)
      (LocalVariables|SetIn%20Weightmap%20Layer%20Name Weightmap%20Layer%20Name))
    (:then_1
      (Utilities|FlowControl|Sequence
        (:then_0
          ;[1 1 1] Check for parameter changes
          (bind _output_get (LocalVariables|SetIs%20Parameter%20Changed (!= (Utilities|Array|Length (Variables|Default|GetAffectedWeightmapLayers)) (Utilities|Array|Length (Variables|Parameters|GetMaterials)))))
          (if (not _output_get)
            (for (_array_element _array_index) (Variables|Parameters|GetMaterials)
              (LocalVariables|SetIs%20Parameter%20Changed (Math|Boolean|ORBoolean (Utilities|Name|NotEqual(Name) (.Name (Utilities|Struct|BreakStruct_LandmassWeightBrushMaterials _array_element)) (Utilities|Array|Get(acopy) (Variables|Default|GetAffectedWeightmapLayers) _array_index)) (!= (.Material (Utilities|Struct|BreakStruct_LandmassWeightBrushMaterials _array_element)) (.Value (Utilities|Map|Find (Variables|Internal|GetMaterials%20by%20Layer) (.Name (Utilities|Struct|BreakStruct_LandmassWeightBrushMaterials _array_element))))) (LocalVariables|GetIs%20Parameter%20Changed))))))
        (:then_1
          (Utilities|FlowControl|Sequence
            (:then_0
              (if (LocalVariables|GetIs%20Parameter%20Changed)
                (Utilities|FlowControl|Sequence
                  (:then_0
                    ;[1 1 1] Set affect-weightmap
                    (Variables|Default|SetAffectWeightmap (> (Utilities|Array|Length (Variables|Parameters|GetMaterials)) 0)))
                  (:then_1
                    (Utilities|FlowControl|Sequence
                      (:then_0
                        ;[1 1 1] Set affected-weightmap-layers
                        (Utilities|Array|Clear _affectedweightmaplayers)
                        (for _array_element_2 (Variables|Parameters|GetMaterials)
                          (Utilities|Array|AddUnique _affectedweightmaplayers (.Name (Utilities|Struct|BreakStruct_LandmassWeightBrushMaterials _array_element_2)))))
                      (:then_1
                        (Utilities|FlowControl|Sequence
                          (:then_0
                            ;[1 1 1] Cache materials by layer name
                            (Utilities|Map|Clear (Variables|Internal|GetMaterials%20by%20Layer))
                            (for _array_element_3 (Variables|Parameters|GetMaterials)
                              (Utilities|Map|Add (Variables|Internal|GetMaterials%20by%20Layer) (.Name (Utilities|Struct|BreakStruct_LandmassWeightBrushMaterials _array_element_3)) (.Material (Utilities|Struct|BreakStruct_LandmassWeightBrushMaterials _array_element_3)))))
                          (:then_1
                            (Utilities|FlowControl|Sequence
                              (:then_0
                                ;[1 1 1] Clear Parameter change flag
                                (LocalVariables|SetIs%20Parameter%20Changed false)))))))))))
            (:then_1
              (Utilities|FlowControl|Sequence
                (:then_0
                  (if (LocalVariables|GetIn%20Is%20Heightmap)
                    (Utilities|FlowControl|Sequence
                      (:then_0
                        ;[1 1 1] Check / Create RT (Something that is lost often)
                        (Utilities|IsValid (Variables|Internal|GetCurrent%20RT)
                          (:Is%20Not%20Valid
                            (Default|EnsureCachedRenderTarget (CallFunction|GetBrushDataManager) self (Variables|Constants|GetRT%20Format) (Utilities|Struct|MakeIntPoint (Variables|/Script/Engine.TextureRenderTarget2D|GetSizeX (LocalVariables|GetIn%20Combined%20Result)) (Variables|/Script/Engine.TextureRenderTarget2D|GetSizeY (LocalVariables|GetIn%20Combined%20Result)))))))
                      (:then_1
                        (Utilities|FlowControl|Sequence
                          (:then_0
                            ;[1 1 1] Check / Create MIDs (Maps themselves are readonly and dont tend to get lost)
                            (bind _values (Utilities|Map|Values (Variables|Internal|GetMaterials%20by%20Layer)))
                            (bind _keys (Utilities|Map|Keys _current_mid_by_material))
                            (bind _values_2 (Utilities|Map|Values _current_mid_by_material))
                            (if (or (not (Utilities|Array|Identical _keys _values)) (Utilities|Array|ContainsItem _values_2 0))
                              (Utilities|Map|Clear _current_mid_by_material)
                              (for _array_element_4 _values
                                (Default|EnsureCachedMID _brush_data_manager _array_element_4)
                                (Utilities|Map|Add _current_mid_by_material _array_element_4 (Default|GetCachedMID _brush_data_manager _array_element_4))))))))))
                (:then_1
                  (Utilities|FlowControl|Sequence
                    (:then_0
                      ;[1 1 1] Set current MID of current Layer
                      (Variables|Internal|SetCurrent%20MID (.Value (Utilities|Map|Find (Variables|Internal|GetCurrent%20MID%20by%20Material) (.Value (Utilities|Map|Find (Variables|Internal|GetMaterials%20by%20Layer) (LocalVariables|GetIn%20Weightmap%20Layer%20Name)))))))
                    (:then_1
                      (Utilities|FlowControl|Sequence
                        (:then_0
                          ;[1 1 1] Set current RT
                          (Variables|Internal|SetCurrent%20RT (Default|GetCachedRenderTarget (CallFunction|GetBrushDataManager) self)))))))))))))))

(fn SetupHeightRelatedMaterialParameters
  (params (Texture%20Render%20Target :type Texture%20Render%20Target%202D%20Object%20Reference%20%28by%20ref%29) (MIDs :type Array%20of%20Material%20Instance%20Dynamic%20Object%20References))
  ;[1 1 1] Parameters
  (for _array_element MIDs
    (Rendering|Material|SetTextureParameterValue _array_element "HeightRT" Texture%20Render%20Target)
    (Rendering|Material|SetVectorParameterValue _array_element "Position" (Math|Conversions|ToLinearColor(Vector) (Transformation|GetActorLocation)) :!class /Script/Engine.MaterialInstanceDynamic)))

(fn SetupWeightRelatedMaterialParameters
  (params (MID :type Material%20Instance%20Dynamic%20Object%20Reference%20%28by%20ref%29))
  ;[1 1 1] Parameters
  (Rendering|Material|SetVectorParameterValue MID "Position" (Math|Conversions|ToLinearColor(Vector) (Transformation|GetActorLocation)) :!class /Script/Engine.MaterialInstanceDynamic))