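; BP_LandmassPatternBrush is a height-only Landmass brush that applies a tiled pattern texture to the heightmap.
; It supplies PatternMaterial as the height-changing material and fills its dynamic instance with the heightmap, pattern texture and tiling.
; Actor location and cached world size from the brush data manager are also passed in.
; Elevation minimum, maximum, pre-offset and invert flag are packed into one vector parameter.
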(fn ConstructionScript)

(fn GetHeight-ChangingMaterial
  ;[1 1 1] Return pattern material
  (return (Variables|Constants|GetPattern%20Material)))

(fn SetMaterialParameters
  (params (MID :type Material%20Instance%20Dynamic%20Object%20Reference%20%28by%20ref%29) (Heightmap :type Texture%20Render%20Target%202D%20Object%20Reference%20%28by%20ref%29))
  (Utilities|FlowControl|Sequence
    (:then_0
      ;[1 1 1] Set Parameters
      (Rendering|Material|SetVectorParameterValue MID "Position" (Math|Conversions|ToLinearColor(Vector) (Transformation|GetActorLocation)) :!class /Script/Engine.MaterialInstanceDynamic)
      (Rendering|Material|SetVectorParameterValue MID "WorldSize" (Math|Conversions|ToLinearColor(Vector) (Default|GetCachedWorldSize (CallFunction|GetBrushDataManager))) :!class /Script/Engine.MaterialInstanceDynamic)
      (Rendering|Material|SetTextureParameterValue MID "HeightRT" Heightmap)
      (Rendering|Material|SetTextureParameterValue MID "PatternTexture" (Variables|Parameters|GetPattern%20Texture))
      (Rendering|Material|SetScalarParameterValue MID "Tiling" (Variables|Parameters|GetPattern%20Tiling) :!class /Script/Engine.MaterialInstanceDynamic)
      (Rendering|Material|SetVectorParameterValue MID "ElevationParams" (Utilities|Struct|MakeLinearColor (Variables|Parameters|GetPattern%20Elevation%20Minimum) (Variables|Parameters|GetPattern%20Elevation%20Maximum) (Variables|Parameters|GetPattern%20Elevation%20Pre-Offset) (Math|Conversions|ToFloat(Boolean) (Variables|Parameters|GetPattern%20Invert%20Elevation))) :!class /Script/Engine.MaterialInstanceDynamic))
    (:then_1
      (Utilities|FlowControl|Sequence
        (:then_0
          ;[1 1 1] End
          (return))))))