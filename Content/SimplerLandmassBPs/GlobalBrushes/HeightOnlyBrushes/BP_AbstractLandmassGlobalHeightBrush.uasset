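; Abstract base landscape brush that alters the whole heightmap through a material supplied by subclasses, leaving weightmaps untouched.
; Subclasses override GetHeightChangingMaterial and SetMaterialParameters, while Render draws the resulting MID into a render target matching the input's size.
; The brush data manager caches MIDs, render targets and landscape world size.
; An update delay throttles redraws by returning the cached target, and an optional debug target mirrors the output.
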(fn ConstructionScript)

(fn Render
  (params (InIsHeightmap :type Boolean) (InCombinedResult :type Texture%20Render%20Target%202D%20Object%20Reference) (InWeightmapLayerName :type Name%20%28by%20ref%29 :default "None"))
  (bind _current_rt (Variables|Default|GetCurrent%20RT))
  (bind _debug_render_target (Variables|Debug|GetDebug%20Render%20Target))
  (Utilities|FlowControl|Sequence
    (:then_0
      ;[1 1 1] Local Variables
      (LocalVariables|SetIn%20Is%20Heightmap InIsHeightmap)
      (LocalVariables|SetIn%20Combined%20Result InCombinedResult))
    (:then_1
      (Utilities|FlowControl|Sequence
        (:then_0
          ;[1 1 1] Set affect-heightmap / affect-weightmap
          (Variables|Default|SetAffectHeightmap true)
          (Variables|Default|SetAffectWeightmap false)
          (Utilities|Array|Clear (Variables|Default|GetAffectedWeightmapLayers)))
        (:then_1
          (Utilities|FlowControl|Sequence
            (:then_0
              ;[1 1 1] Early return for if disabled
              (if (not (Variables|Default|GetIs%20Brush%20Enabled))
                (return (LocalVariables|GetIn%20Combined%20Result))))
            (:then_1
              (Utilities|FlowControl|Sequence
                (:then_0
                  ;[1 1 1] Early return for weightmaps
                  (if (not (LocalVariables|GetIn%20Is%20Heightmap))
                    (return (LocalVariables|GetIn%20Combined%20Result))))
                (:then_1
                  (Utilities|FlowControl|Sequence
                    (:then_0
                      ;[1 1 1] Check parameters
                      (if (not (Utilities|IsValid (CallFunction|GetHeight-ChangingMaterial)))
                        (return (LocalVariables|GetIn%20Combined%20Result))))
                    (:then_1
                      (Utilities|FlowControl|Sequence
                        (:then_0
                          ;[1 1 1] Dont update too often, Return probably existing RT from last time
                          (if (not (CallFunction|IsUpdateDelayPassed))
                            (return (Default|GetCachedRenderTarget (CallFunction|GetBrushDataManager) self))))
                        (:then_1
                          (Utilities|FlowControl|Sequence
                            (:then_0
                              ;[1 1 1] Set internal variables like MID or RT
                              (CallFunction|ResetInternalState (LocalVariables|GetIn%20Combined%20Result)))
                            (:then_1
                              (Utilities|FlowControl|Sequence
                                (:then_0
                                  ;[1 1 1] Set material parameters
                                  (CallFunction|SetMaterialParameters (Variables|Default|GetCurrent%20MID) (LocalVariables|GetIn%20Combined%20Result)))
                                (:then_1
                                  (Utilities|FlowControl|Sequence
                                    (:then_0
                                      ;[1 1 1] Explicit debug messages
                                      (if (not (and (Utilities|IsValid (Variables|Default|GetCurrent%20MID)) (Utilities|IsValid (Variables|Default|GetCurrent%20RT))))
                                        (Development|PrintString (Utilities|String|Append "Invalid state in " (Utilities|GetDisplayName self)) true true "(R=1.000000,G=0.416440,B=0.000000,A=1.000000)")))
                                    (:then_1
                                      (Utilities|FlowControl|Sequence
                                        (:then_0
                                          ;[1 1 1] Draw debug target
                                          (if (Utilities|IsValid _debug_render_target)
                                            (Rendering|ClearRenderTarget2D _debug_render_target)
                                            (Rendering|DrawMaterialtoRenderTarget _debug_render_target (Variables|Default|GetCurrent%20MID))))
                                        (:then_1
                                          (Utilities|FlowControl|Sequence
                                            (:then_0
                                              ;[1 1 1] Draw Height MID
                                              (Rendering|ClearRenderTarget2D _current_rt)
                                              (Rendering|DrawMaterialtoRenderTarget _current_rt (Variables|Default|GetCurrent%20MID)))
                                            (:then_1
                                              (Utilities|FlowControl|Sequence
                                                (:then_0
                                                  ;[1 1 1] End
                                                  (CallFunction|ResetUpdateDelay)
                                                  (return (Variables|Default|GetCurrent%20RT)))))))))))))))))))))))))))

(fn ResetInternalState
  (params (Combined%20Result :type Texture%20Render%20Target%202D%20Object%20Reference%20%28by%20ref%29))
  (bind _brush_data_manager (CallFunction|GetBrushDataManager))
  (Utilities|FlowControl|Sequence
    (:then_0
      ;[1 1 1] Local Variables
      (LocalVariables|SetIn%20Combined%20Result Combined%20Result))
    (:then_1
      (Utilities|FlowControl|Sequence
        (:then_0
          ;[1 1 1] Ensure that a valid MID is available
          (Default|EnsureCachedMID (CallFunction|GetBrushDataManager) (CallFunction|GetHeight-ChangingMaterial)))
        (:then_1
          (Utilities|FlowControl|Sequence
            (:then_0
              ;[1 1 1] Ensure that a valid RT is available
              (if (and (!= (Variables|/Script/Engine.TextureRenderTarget2D|GetSizeX (LocalVariables|GetIn%20Combined%20Result)) 0) (!= (Variables|/Script/Engine.TextureRenderTarget2D|GetSizeY (LocalVariables|GetIn%20Combined%20Result)) 0))
                (Default|EnsureCachedRenderTarget (CallFunction|GetBrushDataManager) self (Variables|Constants|GetRT%20Format) (Utilities|Struct|MakeIntPoint (Variables|/Script/Engine.TextureRenderTarget2D|GetSizeX (LocalVariables|GetIn%20Combined%20Result)) (Variables|/Script/Engine.TextureRenderTarget2D|GetSizeY (LocalVariables|GetIn%20Combined%20Result))))))
            (:then_1
              (Utilities|FlowControl|Sequence
                (:then_0
                  ;[1 1 1] Read RT, MID, etc from Cache
                  (Variables|Default|SetCurrent%20MID (Default|GetCachedMID _brush_data_manager (CallFunction|GetHeight-ChangingMaterial)))
                  (Variables|Default|SetCurrent%20RT (Default|GetCachedRenderTarget _brush_data_manager self)))
                (:then_1
                  (Utilities|FlowControl|Sequence
                    (:then_0
                      ;[1 1 1] End
                      (return))))))))))))

(fn GetHeight-ChangingMaterial
  ;[1 1 1] To be implemented in subclasses. Returns a material that adjusts the heightmap values.
  (return 0))

(fn SetMaterialParameters
  (params (MID :type Material%20Instance%20Dynamic%20Object%20Reference%20%28by%20ref%29) (Heightmap :type Texture%20Render%20Target%202D%20Object%20Reference%20%28by%20ref%29))
  ;[1 1 1] To be implemented in subclasses. The MID is prepared by the this class and this method should be used to set its material parameters.
  (return))

(fn Initialize
  (params (InLandscapeTransform :type Transform%20%28by%20ref%29) (InLandscapeSize :type Int%20Point%20Structure%20%28by%20ref%29) (InLandscapeRenderTargetSize :type Int%20Point%20Structure%20%28by%20ref%29))
  (Utilities|FlowControl|Sequence
    (:then_0
      ;[1 1 1] Local Variables
      (LocalVariables|SetIn%20Landscape%20Transform InLandscapeTransform)
      (LocalVariables|SetIn%20Landscape%20Size InLandscapeSize)
      (LocalVariables|SetIn%20Landscape%20Render%20Target%20Size InLandscapeRenderTargetSize))
    (:then_1
      (Utilities|FlowControl|Sequence
        (:then_0
          ;[1 1 1] Cache World Size
          (Default|CacheWorldSize (CallFunction|GetBrushDataManager) (LocalVariables|GetIn%20Landscape%20Size) (LocalVariables|GetIn%20Landscape%20Transform)))
        (:then_1
          (Utilities|FlowControl|Sequence
            (:then_0
              ;[1 1 1] End
              (return))))))))