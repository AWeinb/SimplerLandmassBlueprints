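; BP_LandmassNoiseBrush is a height-only Landmass brush that applies procedural noise to terrain height through a material.
; It supplies the noise material as its height-changing material, then feeds that material instance the actor location, cached world size from the brush data manager and incoming heightmap.
; Noise shape and elevation settings are packed into vector parameters, while a scalar switches between gradient and Voronoi noise.
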(fn ConstructionScript)

(fn GetHeight-ChangingMaterial
  ;[1 1 1] Return noise material
  (return (Variables|Constants|GetNoise%20Material)))

(fn SetMaterialParameters
  (params (MID :type Material%20Instance%20Dynamic%20Object%20Reference%20%28by%20ref%29) (Heightmap :type Texture%20Render%20Target%202D%20Object%20Reference%20%28by%20ref%29))
  (Utilities|FlowControl|Sequence
    (:then_0
      ;[1 1 1] Set Parameters
      (Rendering|Material|SetVectorParameterValue MID "Position" (Math|Conversions|ToLinearColor(Vector) (Transformation|GetActorLocation)) :!class /Script/Engine.MaterialInstanceDynamic)
      (Rendering|Material|SetVectorParameterValue MID "WorldSize" (Math|Conversions|ToLinearColor(Vector) (Default|GetCachedWorldSize (CallFunction|GetBrushDataManager))) :!class /Script/Engine.MaterialInstanceDynamic)
      (Rendering|Material|SetTextureParameterValue MID "HeightRT" Heightmap)
      (Rendering|Material|SetVectorParameterValue MID "NoiseSeedParams" (Utilities|Struct|MakeLinearColor (Variables|Parameters|GetNoise%20Tiling) (Variables|Parameters|GetNoise%20Seed) (Variables|Parameters|GetNoise%20Octaves) (Variables|Parameters|GetNoise%20Persistence)) :!class /Script/Engine.MaterialInstanceDynamic)
      (Rendering|Material|SetVectorParameterValue MID "ElevationParams" (Utilities|Struct|MakeLinearColor (Variables|Parameters|GetNoise%20Elevation%20Minimum) (Variables|Parameters|GetNoise%20Elevation%20Maximum) (Variables|Parameters|GetNoise%20Elevation%20Pre-Offset) (Math|Conversions|ToFloat(Boolean) (Variables|Parameters|GetNoise%20Invert%20Elevation))) :!class /Script/Engine.MaterialInstanceDynamic)
      (Rendering|Material|SetScalarParameterValue MID "GradientOrVoronoi" (Math|Conversions|ToFloat(Boolean) (Variables|Parameters|GetNoise%20Use%20Voronoi)) :!class /Script/Engine.MaterialInstanceDynamic))
    (:then_1
      (Utilities|FlowControl|Sequence
        (:then_0
          ;[1 1 1] End
          (return))))))