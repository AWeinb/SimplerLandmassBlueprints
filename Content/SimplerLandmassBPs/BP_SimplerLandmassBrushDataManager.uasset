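; Data manager for Simpler Landmass brushes that caches landscape world size, dynamic material instances and render targets.
; Ensure functions create map entries keyed by a parent object, rebuilding render targets on size or format changes and material instances on parent mismatch.
; World size derives from landscape size and transform scale, and getters return the cached values.
; Invalid inputs, failed creation and an unset world size print warnings to screen.
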(fn ConstructionScript)

(fn GetCachedWorldSize
  (bind _cached_world_size (Variables|Cache|GetCached%20World%20Size))
  (bind (_x _y) (Math|Vector|BreakVector _cached_world_size))
  (Utilities|FlowControl|Sequence
    (:then_0
      ;[1 1 1] Comment
      (if (or (== _x 0.0) (== _y 0.0))
        (Development|PrintString (Utilities|String|Append "Invalid Cached World Size in > " (Utilities|GetDisplayName self)) true true "(R=1.000000,G=0.416440,B=0.000000,A=1.000000)")
        (return "0, 0, 0")))
    (:then_1
      (Utilities|FlowControl|Sequence
        (:then_0
          ;[1 1 1] Comment
          (return (Variables|Cache|GetCached%20World%20Size)))))))

(fn GetCachedRenderTarget
  (params (Parent :type Actor%20Object%20Reference))
  ;[1 1 1] Comment
  (return (.Value (Utilities|Map|Find (Variables|Cache|GetCached%20Render%20Targets) Parent))))

(fn GetCachedMID
  (params (Parent :type Material%20Interface%20Object%20Reference%20%28by%20ref%29))
  ;[1 1 1] Comment
  (return (.Value (Utilities|Map|Find (Variables|Cache|GetCached%20MIDs) Parent))))

(fn CacheWorldSize
  (params (Landscape%20Size :type Int%20Point%20Structure) (Landscape%20Transform :type Transform))
  (bind (_x _y) (Utilities|Struct|BreakIntPoint Landscape%20Size))
  (bind _scale (Math|Transform|BreakTransform Landscape%20Transform))
  (bind (_x_2 _y_2) (Math|Vector|BreakVector _scale))
  ;[1 1 1] Compute World Size
  (Variables|Cache|SetCached%20World%20Size (Math|Vector|MakeVector (* (Math|Conversions|ToFloat(Integer) _x) _x_2) (* (Math|Conversions|ToFloat(Integer) _y) _y_2) 0.512)))

(fn EnsureCachedMID
  (params (Parent :type Material%20Interface%20Object%20Reference%20%28by%20ref%29))
  (bind _cached_mids (Variables|Cache|GetCached%20MIDs))
  (Utilities|FlowControl|Sequence
    (:then_0
      ;[1 1 1] Set local Variables
      (LocalVariables|SetIn%20Parent Parent))
    (:then_1
      (Utilities|FlowControl|Sequence
        (:then_0
          ;[1 1 1] Check parameters
          (if (not (Utilities|IsValid (LocalVariables|GetIn%20Parent)))
            (Development|PrintString (Utilities|String|Append "Invalid Input in " (Utilities|GetDisplayName self)) true true "(R=1.000000,G=0.416440,B=0.000000,A=1.000000)")
            (return)))
        (:then_1
          (Utilities|FlowControl|Sequence
            (:then_0
              ;[1 1 1] Check / Create MID
              (Utilities|IsValid (.Value (Utilities|Map|Find _cached_mids (LocalVariables|GetIn%20Parent)))
                (:Is%20Valid
                  (if (not (== (LocalVariables|GetIn%20Parent) (Variables|/Script/Engine.MaterialInstance|GetParent (.Value (Utilities|Map|Find _cached_mids (LocalVariables|GetIn%20Parent))))))
                    (bind _returnvalue (Rendering|Material|CreateDynamicMaterialInstance (LocalVariables|GetIn%20Parent) "None" "None" :!class /Script/Engine.KismetMaterialLibrary :!label _label))
                    (Utilities|Map|Add _cached_mids (LocalVariables|GetIn%20Parent) _returnvalue)))
                (:Is%20Not%20Valid
                  (goto _label))))
            (:then_1
              (Utilities|FlowControl|Sequence
                (:then_0
                  ;[1 1 1] Validate MID
                  (Utilities|IsValid (.Value (Utilities|Map|Find (Variables|Cache|GetCached%20MIDs) (LocalVariables|GetIn%20Parent)))
                    (:Is%20Not%20Valid
                      (Development|PrintString (Utilities|String|Append "Failure creating MID for " (Utilities|GetDisplayName (LocalVariables|GetIn%20Parent))) true true "(R=1.000000,G=0.416440,B=0.000000,A=1.000000)"))))
                (:then_1
                  (Utilities|FlowControl|Sequence
                    (:then_0
                      ;[1 1 1] Return
                      (return))))))))))))

(fn EnsureCachedRenderTarget
  (params (Parent :type Actor%20Object%20Reference) (Format :type ETextureRenderTargetFormat%20Enum :default "RTF_R8") (Size :type Int%20Point%20Structure))
  (Utilities|FlowControl|Sequence
    (:then_0
      ;[1 1 1] Set local Variables
      (LocalVariables|SetIn%20Parent Parent)
      (LocalVariables|SetIn%20Format Format)
      (LocalVariables|SetIn%20Size Size))
    (:then_1
      (Utilities|FlowControl|Sequence
        (:then_0
          ;[1 1 1] Check Parameters with early return
          (if (Utilities|IsValid (LocalVariables|GetIn%20Parent))
            (if (not (and (!= (.X (Utilities|Struct|BreakIntPoint (LocalVariables|GetIn%20Size))) 0) (!= (.Y (Utilities|Struct|BreakIntPoint (LocalVariables|GetIn%20Size))) 0)))
              (Development|PrintString (Utilities|String|Append "Invalid Input in " (Utilities|GetDisplayName self)) true true "(R=1.000000,G=0.416440,B=0.000000,A=1.000000)" :!label _label)
              (return))
            (else
              (goto _label))))
        (:then_1
          (Utilities|FlowControl|Sequence
            (:then_0
              ;[1 1 1] Control / Create RT
              (Utilities|IsValid (.Value (Utilities|Map|Find (Variables|Cache|GetCached%20Render%20Targets) (LocalVariables|GetIn%20Parent)))
                (:Is%20Valid
                  (if (not (Math|Boolean|ANDBoolean (== (Variables|/Script/Engine.TextureRenderTarget2D|GetSizeX (.Value (Utilities|Map|Find (Variables|Cache|GetCached%20Render%20Targets) (LocalVariables|GetIn%20Parent)))) (.X (Utilities|Struct|BreakIntPoint (LocalVariables|GetIn%20Size)))) (== (Variables|/Script/Engine.TextureRenderTarget2D|GetSizeY (.Value (Utilities|Map|Find (Variables|Cache|GetCached%20Render%20Targets) (LocalVariables|GetIn%20Parent)))) (.Y (Utilities|Struct|BreakIntPoint (LocalVariables|GetIn%20Size)))) (Utilities|Enum|Equal(Enum) (LocalVariables|GetIn%20Format) (Variables|/Script/Engine.TextureRenderTarget2D|GetRenderTargetFormat (.Value (Utilities|Map|Find (Variables|Cache|GetCached%20Render%20Targets) (LocalVariables|GetIn%20Parent)))))))
                    (bind _returnvalue (Rendering|CreateRenderTarget2D (.X (Utilities|Struct|BreakIntPoint (LocalVariables|GetIn%20Size))) (.Y (Utilities|Struct|BreakIntPoint (LocalVariables|GetIn%20Size))) (LocalVariables|GetIn%20Format) :!label _label_2))
                    (LocalVariables|SetCreated%20RT _returnvalue)))
                (:Is%20Not%20Valid
                  (goto _label_2))))
            (:then_1
              (Utilities|FlowControl|Sequence
                (:then_0
                  ;[1 1 1] Store new RT
                  (Utilities|IsValid (LocalVariables|GetCreated%20RT)
                    (:Is%20Valid
                      (Utilities|Map|Remove (Variables|Cache|GetCached%20Render%20Targets) (LocalVariables|GetIn%20Parent))
                      (Utilities|Map|Add (Variables|Cache|GetCached%20Render%20Targets) (LocalVariables|GetIn%20Parent) (LocalVariables|GetCreated%20RT)))))
                (:then_1
                  (Utilities|FlowControl|Sequence
                    (:then_0
                      ;[1 1 1] Validate RT
                      (Utilities|IsValid (.Value (Utilities|Map|Find (Variables|Cache|GetCached%20Render%20Targets) (LocalVariables|GetIn%20Parent)))
                        (:Is%20Not%20Valid
                          (Development|PrintString (Utilities|String|Append "Failure creating RT for " (Utilities|GetDisplayName (LocalVariables|GetIn%20Parent))) true true "(R=1.000000,G=0.416440,B=0.000000,A=1.000000)"))))
                    (:then_1
                      (Utilities|FlowControl|Sequence
                        (:then_0
                          ;[1 1 1] Return
                          (return))))))))))))))