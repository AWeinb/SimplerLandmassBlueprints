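; Landmass landscape brush that applies a tiled pattern texture to the landscape heightmap through a material, ignoring weightmaps.
; Initialize caches the landscape's world size in a BrushDataManager, which also provides the cached material instance and render target.
; Render feeds the incoming height target, actor position, world size, tiling and elevation settings into the material, then draws and returns the result.
; An optional debug render target receives the same draw.
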(fn ConstructionScript)

(fn Initialize
  (params (InLandscapeTransform :type Transform%20%28by%20ref%29) (InLandscapeSize :type Int%20Point%20Structure%20%28by%20ref%29) (InLandscapeRenderTargetSize :type Int%20Point%20Structure%20%28by%20ref%29))
  (Utilities|FlowControl|Sequence
    (:then_0
      ;[1 1 1] Set local variables
      (LocalVariables|SetIn%20Landscape%20Transform InLandscapeTransform)
      (LocalVariables|SetIn%20Landscape%20Size InLandscapeSize)
      (LocalVariables|SetIn%20Landscape%20Render%20Target%20Size InLandscapeRenderTargetSize))
    (:then_1
      (Utilities|FlowControl|Sequence
        (:then_0
          ;[1 1 1] Initialize Brush Data Manager
          (Utilities|IsValid (Variables|Internal|GetBrush%20Data%20Manager)
            (:Is%20Not%20Valid
              (bind _brush_data_manager (CallFunction|EnsureBrushDataManager))
              (Variables|Internal|SetBrush%20Data%20Manager _brush_data_manager))))
        (:then_1
          (Utilities|FlowControl|Sequence
            (:then_0
              ;[1 1 1] Cache World Size
              (Default|CacheWorldSize (Variables|Internal|GetBrush%20Data%20Manager) (LocalVariables|GetIn%20Landscape%20Size) (LocalVariables|GetIn%20Landscape%20Transform)))))))))

(fn Render
  (params (InIsHeightmap :type Boolean) (InCombinedResult :type Texture%20Render%20Target%202D%20Object%20Reference) (InWeightmapLayerName :type Name%20%28by%20ref%29 :default "None"))
  (bind _debug_render_target (Variables|Debug|GetDebug%20Render%20Target))
  (Utilities|FlowControl|Sequence
    (:then_0
      ;[1 1 1] Local Variables
      (bind _output_get (LocalVariables|SetIn%20Is%20Heightmap InIsHeightmap))
      (if _output_get
        (LocalVariables|SetIn%20Landscape%20Render%20Target InCombinedResult)))
    (:then_1
      (Utilities|FlowControl|Sequence
        (:then_0
          ;[1 1 1] Set affect-heightmap / affect-weightmap
          (Variables|Default|SetAffectHeightmap true)
          (Variables|Default|SetAffectWeightmap false)
          (Utilities|Array|Clear (Variables|Default|GetAffectedWeightmapLayers)))
        (:then_1
          (Utilities|FlowControl|Sequence
            (:then_0
              ;[1 1 1] Early return for weightmaps
              (if (not (LocalVariables|GetIn%20Is%20Heightmap))
                (return 0)))
            (:then_1
              (Utilities|FlowControl|Sequence
                (:then_0
                  ;[1 1 1] Check parameters
                  (if (not (Utilities|IsValid (Variables|Constants|GetPattern%20Material)))
                    (return (LocalVariables|GetIn%20Landscape%20Render%20Target))))
                (:then_1
                  (Utilities|FlowControl|Sequence
                    (:then_0
                      ;[1 1 1] Get Brush Data Manager
                      (Utilities|IsValid (Variables|Internal|GetBrush%20Data%20Manager)
                        (:Is%20Valid
                          _)
                        (:Is%20Not%20Valid
                          (bind _brush_data_manager (CallFunction|EnsureBrushDataManager))
                          (Variables|Internal|SetBrush%20Data%20Manager _brush_data_manager)))
                      (Utilities|FlowControl|Sequence
                        (:then_0
                          ;[1 1 1] Ensure that a valid MID is available
                          (Default|EnsureCachedMID (Variables|Internal|GetBrush%20Data%20Manager) (Variables|Constants|GetPattern%20Material)))
                        (:then_1
                          (Utilities|FlowControl|Sequence
                            (:then_0
                              ;[1 1 1] Ensure that a valid RT is available
                              (if (and (!= (Variables|/Script/Engine.TextureRenderTarget2D|GetSizeX (LocalVariables|GetIn%20Landscape%20Render%20Target)) 0) (!= (Variables|/Script/Engine.TextureRenderTarget2D|GetSizeY (LocalVariables|GetIn%20Landscape%20Render%20Target)) 0))
                                (Default|EnsureCachedRenderTarget (Variables|Internal|GetBrush%20Data%20Manager) self (Variables|Constants|GetRT%20Format) (Utilities|Struct|MakeIntPoint (Variables|/Script/Engine.TextureRenderTarget2D|GetSizeX (LocalVariables|GetIn%20Landscape%20Render%20Target)) (Variables|/Script/Engine.TextureRenderTarget2D|GetSizeY (LocalVariables|GetIn%20Landscape%20Render%20Target))))))
                            (:then_1
                              (Utilities|FlowControl|Sequence
                                (:then_0
                                  ;[1 1 1] Read RT, MID, etc from Cache
                                  (Variables|Internal|SetCurrent%20World%20Size (Default|GetCachedWorldSize (Variables|Internal|GetBrush%20Data%20Manager)))
                                  (Variables|Internal|SetCurrent%20MID (Default|GetCachedMID (Variables|Internal|GetBrush%20Data%20Manager) (Variables|Constants|GetPattern%20Material)))
                                  (Variables|Internal|SetCurrent%20RT (Default|GetCachedRenderTarget (Variables|Internal|GetBrush%20Data%20Manager) self)))
                                (:then_1
                                  (Utilities|FlowControl|Sequence
                                    (:then_0
                                      ;[1 1 1] Set material parameters
                                      (CallFunction|SetupMaterialParameters (Variables|Internal|GetCurrent%20MID) (LocalVariables|GetIn%20Landscape%20Render%20Target) (Variables|Internal|GetCurrent%20World%20Size)))
                                    (:then_1
                                      (Utilities|FlowControl|Sequence
                                        (:then_0
                                          ;[1 1 1] Explicit debug messages
                                          (if (not (and (Utilities|IsValid (Variables|Internal|GetCurrent%20MID)) (Utilities|IsValid (Variables|Internal|GetCurrent%20RT))))
                                            (Development|PrintString (Utilities|String|Append "Invalid state in " (Utilities|GetDisplayName self)) true true "(R=1.000000,G=0.416440,B=0.000000,A=1.000000)")))
                                        (:then_1
                                          (Utilities|FlowControl|Sequence
                                            (:then_0
                                              ;[1 1 1] Draw debug target
                                              (if (Utilities|IsValid _debug_render_target)
                                                (Rendering|ClearRenderTarget2D _debug_render_target)
                                                (Rendering|DrawMaterialtoRenderTarget _debug_render_target (Variables|Internal|GetCurrent%20MID))))
                                            (:then_1
                                              (Utilities|FlowControl|Sequence
                                                (:then_0
                                                  ;[1 1 1] Draw Height MID
                                                  (Rendering|ClearRenderTarget2D (Variables|Internal|GetCurrent%20RT))
                                                  (Rendering|DrawMaterialtoRenderTarget (Variables|Internal|GetCurrent%20RT) (Variables|Internal|GetCurrent%20MID))
                                                  (return (Variables|Internal|GetCurrent%20RT)))))))))))))))))))))))))))

(fn SetupMaterialParameters
  (params (MID :type Material%20Instance%20Dynamic%20Object%20Reference%20%28by%20ref%29) (HeightRT :type Texture%20Render%20Target%202D%20Object%20Reference%20%28by%20ref%29) (World%20Size :type Vector))
  ;[1 1 1] Parameters
  (Rendering|Material|SetVectorParameterValue MID "Position" (Math|Conversions|ToLinearColor(Vector) (Transformation|GetActorLocation)) :!class /Script/Engine.MaterialInstanceDynamic)
  (Rendering|Material|SetVectorParameterValue MID "WorldSize" (Math|Conversions|ToLinearColor(Vector) World%20Size) :!class /Script/Engine.MaterialInstanceDynamic)
  (Rendering|Material|SetTextureParameterValue MID "HeightRT" HeightRT)
  (Rendering|Material|SetTextureParameterValue MID "PatternTexture" (Variables|Parameters|GetPattern%20Texture))
  (Rendering|Material|SetScalarParameterValue MID "Tiling" (Variables|Parameters|GetPattern%20Tiling) :!class /Script/Engine.MaterialInstanceDynamic)
  (Rendering|Material|SetVectorParameterValue MID "ElevationParams" (Utilities|Struct|MakeLinearColor (Variables|Parameters|GetPattern%20Elevation%20Minimum) (Variables|Parameters|GetPattern%20Elevation%20Maximum) (Variables|Parameters|GetPattern%20Elevation%20Pre-Offset) (Math|Conversions|ToFloat(Boolean) (Variables|Parameters|GetPattern%20Invert%20Elevation))) :!class /Script/Engine.MaterialInstanceDynamic))